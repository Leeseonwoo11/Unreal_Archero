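; BP_NoMonsterMap is a map Blueprint, named for a stage without monsters, that provides the portal to the next stage.
; It caches the ABGameInstance on BeginPlay.
; When a component tagged PLAYER begins overlapping Potal, it increments the Stage stored in that game instance and opens ThirdPersonExampleMap, so stage progress persists across the level load.
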(event `self.ReceiveBeginPlay`
  ;[1 1 1] BeginPlay
  (bind _asabgame_instance (cast `ABGameInstance` (`GameplayStatics.GetGameInstance`)))
  (set `self.ABGameInstance` _asabgame_instance))

(event `self.potal.OnComponentBeginOverlap`
  (params (OverlappedComponent :type "PrimitiveComponent Object Reference") (OtherActor :type "Actor Object Reference") (OtherComp :type "PrimitiveComponent Object Reference") (OtherBodyIndex :type Integer) (bFromSweep :type Boolean) (SweepResult :type "HitResult Structure (by ref)"))
  (bind _abgameinstance (`self.ABGameInstance`))
  ;[1 1 1] 다음레벨 포탈설정
  (if (`ActorComponent.ComponentHasTag` OtherComp "PLAYER")
    (set `ABGameInstance.Stage` (+ (`ABGameInstance.Stage` _abgameinstance) 1) _abgameinstance)
    (`GameplayStatics.OpenLevel` "ThirdPersonExampleMap")))

(fn `UserConstructionScript`)