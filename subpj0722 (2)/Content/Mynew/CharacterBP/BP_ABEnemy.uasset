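; Enemy character Blueprint that chases the player, reacts to arrow hits and shows an HP bar.
; BeginPlay attaches meshes to both hand sockets and caches the widget's progress bar.
; Tick updates the bar against initially captured HP, rotates it toward a look location, then after a Delay calls Attack, which issues AI MoveTo toward the player.
; "ARROW"-tagged capsule overlaps set the AnimBP hit flag; Attack clears it instead of moving.
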(event `self.ReceiveBeginPlay`
  ;[1 1 1] 코멘트
  (`self.SetWeapon` null)
  (`self.FindEnemyHP`))

(event `self.ReceiveTick`
  (params (DeltaSeconds :type "Float (single-precision)"))
  ;[1 1 1] 코멘트
  (`self.SetHP`)
  (`KismetSystemLibrary.Delay` 3.0)
  (`self.Attack`))

(event `Attack`
  (bind _returnvalue (`AIBlueprintHelperLibrary.GetAIController` (`PawnMovementComponent.GetPawnOwner` (`self.CharacterMovement`))))
  ;[1 1 1] 적공격과 적애니메이션 히트모션 false 셋
  (if (`self.BPISHIT`)
    (bind _output_get (set `self.BPISHIT` false))
    (set `/Game/Mynew/EnemyAnim/ABEnemyAnimBlueprint.ISHIT` _output_get (`self.ABEnemyAnimBlueprint`))
    (else
      (`/Engine/EditorBlueprintResources/StandardMacros.IsValid` _returnvalue
        (:`Is Valid`
          (bind _output_get_2 (set `self.Goal` (`self.K2_GetActorLocation` (`GameplayStatics.GetPlayerCharacter` 0))))
          (`AIController.MoveToLocation` _returnvalue _output_get_2 10.0 true true false true null true))))))

(event `SetWeapon`
  (params (Owner :type "Actor Object Reference"))
  (bind _mesh (`self.Mesh`))
  ;[1 1 1] 무기장착하기
  (`SceneComponent.K2_AttachToComponent` (`self.StaticMesh1`) _mesh "hand_lSocket" "KeepRelative" "KeepRelative" "KeepRelative" true)
  (`SceneComponent.K2_AttachToComponent` (`self.StaticMesh`) _mesh "hand_rSocket" "KeepRelative" "KeepRelative" "KeepRelative" true))

(event `FindEnemyHP`
  ;[1 1 1] BP_EnemyHP 형변환 뒤 변수화
  (bind _asbp_enemy_hp (cast `/Game/Mynew/EnemyHUD/BP_EnemyHP` (`WidgetComponent.GetUserWidgetObject` (`self.Widget1`))))
  (set `self.ProgressBar` (`/Game/Mynew/EnemyHUD/BP_EnemyHP.ProgressBar_107` _asbp_enemy_hp)))

(event `self.CapsuleComponent.OnComponentBeginOverlap`
  (params (OverlappedComponent :type "PrimitiveComponent Object Reference") (OtherActor :type "Actor Object Reference") (OtherComp :type "PrimitiveComponent Object Reference") (OtherBodyIndex :type Integer) (bFromSweep :type Boolean) (SweepResult :type "HitResult Structure (by ref)"))
  ;[1 1 1] 화살에 맞는다면 에님 hit 체크
  (if (`self.ActorHasTag` OtherActor "ARROW")
    (bind _output_get (set `self.BPISHIT` true))
    (bind _asabenemy_anim_blueprint (cast `/Game/Mynew/EnemyAnim/ABEnemyAnimBlueprint` (`SkeletalMeshComponent.GetAnimInstance` (`self.Mesh`))))
    (bind _output_get_2 (set `self.ABEnemyAnimBlueprint` _asabenemy_anim_blueprint))
    (set `/Game/Mynew/EnemyAnim/ABEnemyAnimBlueprint.ISHIT` _output_get _output_get_2)))

(event `SetHP`
  (bind _scene (`self.Scene`))
  (bind _fullhealth (`self.FullHealth`))
  (bind _hp (`self.HP`))
  ;[1 1 1] Enemy HP Percent 설정
  (`|ExecutionSequence`
    (:`then_0`
      (`/Engine/EditorBlueprintResources/StandardMacros.DoOnce` false
        (:`Completed`
          (set `self.FullHealth` _hp))))
    (:`then_1`
      (bind _output_get (set `self.Health` _hp))
      (if (>= _fullhealth 0.1)
        (`ProgressBar.SetPercent` (`self.ProgressBar`) (/ _output_get _fullhealth))
        ;;[1 1 1] Set Widget Rotation
        (`SceneComponent.K2_SetWorldRotation` _scene (`KismetMathLibrary.FindLookAtRotation` (`SceneComponent.K2_GetComponentLocation` _scene) (`self.HpLookLocation`)) false false)))))

(fn `UserConstructionScript`)