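; BP_ACEnemy is an AI enemy character that fires magic balls and roams to random points around the player.
; Tick updates health and death state, then a Delay paces the attack-and-move cycle to roughly every three seconds.
; Hit, attack and death flags drive the animation Blueprint, with "ARROW"-tagged overlaps setting the hit flag.
; A widget health bar shows HP against its first recorded value and rotates toward HpLookLocation.
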(event `self.ReceiveBeginPlay`
  (`self.SetWeapon`)
  (`self.Set BP_ACEnemy Property`)
  (`self.SpawnDefaultController`))

(event `self.CapsuleComponent.OnComponentBeginOverlap`
  (params (OverlappedComponent :type "PrimitiveComponent Object Reference") (OtherActor :type "Actor Object Reference") (OtherComp :type "PrimitiveComponent Object Reference") (OtherBodyIndex :type Integer) (bFromSweep :type Boolean) (SweepResult :type "HitResult Structure (by ref)"))
  ;[1 1 1] ACEnemy AnimHitCheck true
  (if (`self.ActorHasTag` OtherActor "ARROW")
    (bind _output_get (set `self.BP_ISHIT` true))
    (set `/Game/Mynew/EnemyAnim/ACEnemyAnimBlueprint.IsHit` _output_get (`self.BP_AnimACEnemy`))))

(event `self.ReceiveTick`
  (params (DeltaSeconds :type "Float (single-precision)"))
  (`self.Set HP`)
  (`self.Dead Check`)
  (`KismetSystemLibrary.Delay` 3.0)
  (`self.Attack`)
  (`self.MOVE`)
  (`self.TickTail`))

(event `MOVE`
  (bind _returnvalue (`KismetMathLibrary.RandomFloatInRange` -1000.0 1000.0))
  (bind (_returnvalue_x _returnvalue_y) (`KismetMathLibrary.BreakVector` (`self.K2_GetActorLocation` (`GameplayStatics.GetPlayerCharacter` 0))))
  (bind _returnvalue_2 (`AIBlueprintHelperLibrary.GetAIController` (`PawnMovementComponent.GetPawnOwner` (`self.CharacterMovement`))))
  ;[1 1 1] Enemy move to Location( around player Character Location)
  (if (not (<= (`self.Health`) 0.0))
    (`/Engine/EditorBlueprintResources/StandardMacros.IsValid` _returnvalue_2
      (:`Is Valid`
        (`AIController.MoveToLocation` _returnvalue_2 (`KismetMathLibrary.MakeVector` (+ _returnvalue_x _returnvalue) (- _returnvalue_y _returnvalue)) 10.0 true true false true null true)
        ;[1 1 1] After move Set AnimHitCheck false
        (bind _output_get (set `self.BP_ISHIT` false))
        (set `/Game/Mynew/EnemyAnim/ACEnemyAnimBlueprint.IsHit` _output_get (`self.BP_AnimACEnemy`))))))

(event `TickTail`
  ;[1 1 1] Attack check in AnimBlueprint
  (set `/Game/Mynew/EnemyAnim/ACEnemyAnimBlueprint.IsAttack` false (`self.BP_AnimACEnemy`)))

(event `Attack`
  ;[1 1 1] Attack check in AnimBlueprint
  (if (not (<= (`self.Health`) 0.0))
    (`self.MagicBallFire`)
    (set `/Game/Mynew/EnemyAnim/ACEnemyAnimBlueprint.IsAttack` true (`self.BP_AnimACEnemy`))))

(event `SetWeapon`
  ;[1 1 1] 무기장착
  (`SceneComponent.K2_AttachToComponent` (`self.StaticMesh`) (`self.Mesh`) "hand_rSocket" "KeepRelative" "KeepRelative" "KeepRelative" true))

(event `Set HP`
  (bind _scene (`self.Scene`))
  (bind _fullhealth (`self.FullHealth`))
  ;[1 1 1] AC_Enemy HP 관리
  (`|ExecutionSequence`
    (:`then_0`
      (`/Engine/EditorBlueprintResources/StandardMacros.DoOnce` false
        (:`Completed`
          (set `self.FullHealth` (`self.HP`)))))
    (:`then_1`
      (set `self.Health` (`self.HP`))
      (if (>= _fullhealth 0.1)
        (`ProgressBar.SetPercent` (`/Game/Mynew/EnemyHUD/BP_EnemyHP.ProgressBar_107` (`self.BP_EnemyWidget`)) (/ (`self.Health`) _fullhealth))
        (`SceneComponent.K2_SetWorldRotation` _scene (`KismetMathLibrary.FindLookAtRotation` (`SceneComponent.K2_GetComponentLocation` _scene) (`self.HpLookLocation`)) false false)))))

(event `Dead Check`
  ;[1 1 1] 사망체크
  (set `/Game/Mynew/EnemyAnim/ACEnemyAnimBlueprint.IsDead` (<= (`self.Health`) 0.0) (`self.BP_AnimACEnemy`)))

(event `Set BP_ACEnemy Property`
  ;[1 1 1] BP_ACEnemy AnimBlueprint 변수화
  (bind _asacenemy_anim_blueprint (cast `/Game/Mynew/EnemyAnim/ACEnemyAnimBlueprint` (`SkeletalMeshComponent.GetAnimInstance` (`self.Mesh`))))
  (set `self.BP_AnimACEnemy` _asacenemy_anim_blueprint)
  ;[1 1 1] BP_EnemyHP 변수화
  (bind _asbp_enemy_hp (cast `/Game/Mynew/EnemyHUD/BP_EnemyHP` (`WidgetComponent.GetUserWidgetObject` (`self.Widget`))))
  (set `self.BP_EnemyWidget` _asbp_enemy_hp))

(fn `UserConstructionScript`)