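; Boss character Blueprint that carries two attached meshes and shows an on-screen health bar while active.
; BeginPlay attaches the static meshes to the left-hand and backpack sockets of the skeletal mesh.
; While active, Tick creates the BP_BossHP widget once and updates its progress bar from BossHP relative to the first value captured as full health.
; The zero-HP check on Tick triggers nothing.
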(event `self.ReceiveBeginPlay`
  ;[1 1 1] BeginPlay
  (`SceneComponent.K2_AttachToComponent` (`self.StaticMesh`) (`self.Mesh`) "hand_lSocket" "KeepRelative" "KeepRelative" "KeepRelative" true)
  (`SceneComponent.K2_AttachToComponent` (`self.StaticMesh1`) (`self.Mesh`) "Backpack" "KeepRelative" "KeepRelative" "KeepRelative" true))

(event `self.ReceiveTick`
  (params (DeltaSeconds :type "Float (single-precision)"))
  ;[1 1 1] Tick
  (bind _returnvalue (`self.IsActive`))
  (if _returnvalue
    (`|ExecutionSequence`
      (:`then_0`
        (`/Engine/EditorBlueprintResources/StandardMacros.DoOnce` false
          (:`Completed`
            (`self.SetWidget`))))
      (:`then_1`
        (`self.SetBossHP`)
        (if (<= (`self.BossHP`) 0.0)
          _)))))

(event `SetBossHP`
  (bind _bosshp (`self.BossHP`))
  (bind _fullhealth (`self.FullHealth`))
  ;[1 1 1] 보스 HP설정
  (`|ExecutionSequence`
    (:`then_0`
      (`/Engine/EditorBlueprintResources/StandardMacros.DoOnce` false
        (:`Completed`
          (set `self.FullHealth` _bosshp))))
    (:`then_1`
      (bind _output_get (set `self.Health` _bosshp))
      (if (>= _fullhealth 0.1)
        (`ProgressBar.SetPercent` (`/Game/Mynew/EnemyHUD/BP_BossHP.ProgressBar_54` (`self.Bp_BossHPWidget`)) (/ _output_get _fullhealth))))))

(event `SetWidget`
  ;[1 1 1] 위젯설정
  (bind _returnvalue (`|CreateWidget` "/Game/Mynew/EnemyHUD/BP_BossHP.BP_BossHP_C"))
  (bind _output_get (set `self.Bp_BossHPWidget` _returnvalue))
  (`UserWidget.AddToViewport` _output_get 0))

(fn `UserConstructionScript`)